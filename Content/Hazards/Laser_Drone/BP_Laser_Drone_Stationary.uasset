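; Laser drone hazard that fires a continuous beam from its muzzle and damages whatever blocks it.
; Tick spawns the beam particle once, then re-aims it along the muzzle's forward vector each frame.
; A visibility line trace shortens the beam to the hit point and applies damage on every blocked tick.
; The construction script configures InterpToMovement from Location1 and a duration variable; the Location2 point is left unconnected.
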(event `self.ReceiveTick`
  (params (DeltaSeconds :type "Float (single-precision)"))
  (bind _laser_muzzle (`self.Laser_Muzzle`))
  (bind _returnvalue (`SceneComponent.K2_GetComponentLocation` _laser_muzzle))
  (`|ExecutionSequence`
    (:`then_0`
      (`/Engine/EditorBlueprintResources/StandardMacros.DoOnce` false
        (:`Completed`
          (bind _returnvalue_2 (`GameplayStatics.SpawnEmitterAttached` "/Game/Hazards/Laser_Drone/P_Laser.P_Laser" (`self.Laser_Muzzle`) "None" (0.0 0.0 0.0) (struct) (20.0 20.0 20.0)))
          (set `self.Laser` _returnvalue_2))))
    (:`then_1`
      (`ParticleSystemComponent.SetBeamSourcePoint` (`self.Laser`) 0 _returnvalue 0)
      (set `self.Laser_Start_Point` _returnvalue)
      (set `self.Laser_Max_Range_Endpoint` (+ _returnvalue (* (`SceneComponent.GetForwardVector` _laser_muzzle) 5000.0))))
    (:`then_2`
      (bind _outhit (`KismetSystemLibrary.LineTraceSingle` (`self.Laser_Start_Point`) (`self.Laser_Max_Range_Endpoint`) "TraceTypeQuery1"))
      (if (`GameplayStatics.BreakHitResult` _outhit)
        (set `self.Laser_Max_Range_Endpoint` (`.Location` (`GameplayStatics.BreakHitResult` _outhit)))
        (`GameplayStatics.ApplyDamage` (`.HitActor` (`GameplayStatics.BreakHitResult` _outhit)) 30.0 null self))
      (`ParticleSystemComponent.SetBeamEndPoint` (`self.Laser`) 0 (`self.Laser_Max_Range_Endpoint`)))))

(fn `UserConstructionScript`
  (bind _interptomovement (`self.InterpToMovement`))
  (set `InterpToMovementComponent.ControlPoints` (`|MakeArray` (make `InterpControlPoint` (`self.Location_1`)) (struct)) _interptomovement)
  (set `InterpToMovementComponent.Duration` (`self.Control_Point_Move_Duration`) _interptomovement))