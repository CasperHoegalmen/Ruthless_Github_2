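; BP_Wrist_Blade is the player's wrist-mounted melee weapon, which damages Unity Rebel enemies during swipes.
; When its Hitbox begins overlapping an actor tagged Enemy, it checks the player character's MeleeSwiping flag, then calls TakeDamage on the BP_Unity_Rebel with MeleeDamage.
; A Reset_Weapon event reactivates the Weapon component with a reset.
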(event `Reset_Weapon`
  (`ActorComponent.Activate` (`self.Weapon`) true))

(event `self.Hitbox.OnComponentBeginOverlap`
  (params (OverlappedComponent :type "PrimitiveComponent Object Reference") (OtherActor :type "Actor Object Reference") (OtherComp :type "PrimitiveComponent Object Reference") (OtherBodyIndex :type Integer) (bFromSweep :type Boolean) (SweepResult :type "HitResult Structure (by ref)"))
  (if (`self.ActorHasTag` OtherActor "Enemy")
    (bind _asfirst_person_character (cast `/Game/Player_Character/Blueprints/BP_Player_Character` (`GameplayStatics.GetPlayerCharacter` 0)))
    (if (`/Game/Player_Character/Blueprints/BP_Player_Character.Melee_Swiping?` _asfirst_person_character)
      (bind _asbp_unity_rebel (cast `/Game/Enemies/Unity_Rebel/BP_Unity_Rebel` OtherActor))
      (`/Game/Enemies/Unity_Rebel/BP_Unity_Rebel.Take_Damage` _asbp_unity_rebel (`self.Melee_Damage`)))))

(fn `UserConstructionScript`)