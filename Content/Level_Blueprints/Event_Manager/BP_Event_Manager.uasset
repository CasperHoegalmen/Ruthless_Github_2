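; BP_Event_Manager is a level event actor handling player power drain, damage, victory and tutorial popups.
; A Tick gate calls the player's PowerDrain, while other events apply fixed damage or show the victory widget with UI-only input.
; Popup functions add tutorial widgets, pause the game and enable this actor's input.
; Releasing E removes widgets implementing Int_Tutorial_Interface, disables that input and toggles pause.
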(event `self.ReceiveBeginPlay`
  (set `self.Player_Ref` (`GameplayStatics.GetPlayerController` 0))
  (bind _asbp_player_character (cast `/Game/Player_Character/Blueprints/BP_Player_Character` (`GameplayStatics.GetPlayerPawn` 0)))
  (set `self.Player_Actor_Ref` _asbp_player_character))

(event `self.ReceiveTick`
  (params (DeltaSeconds :type "Float (single-precision)"))
  (`/Engine/EditorBlueprintResources/StandardMacros.Gate` true :!label _label
    (:`Exit`
      (`/Game/Player_Character/Blueprints/BP_Player_Character.Power_Drain` (`self.Player_Actor_Ref`)))))

(event `Toggle_Power_Drain`
  (params (New_Power_Drain_Setting :type Boolean))
  (if true
    (goto _label :!via `Open`)
    (else
      (goto _label :!via `Close`))))

(event `Damage_Player`
  (`GameplayStatics.ApplyDamage` (`self.Player_Actor_Ref`) 15.0 null self))

(event `Win_Game`
  (bind _returnvalue (`|CreateWidget` "/Game/Interface/DARK_SCIFI_UI/Widgets/WB_Victory.WB_Victory_C" (`self.Player_Ref`)))
  (`UserWidget.AddToViewport` _returnvalue 0)
  (`WidgetBlueprintLibrary.SetInputMode_UIOnlyEx` (`self.Player_Ref`) _returnvalue))

(event `Toggle_Tutorial`
  (params (`Tutorial_Active?` :type Boolean))
  (if `Tutorial_Active?`
    (if (`self.Power_Drain_Active?`)
      (set `self.Power_Drain_Active?` false)
      (set `self.Power_Drain_To_Resume?` true))
    (`self.EnableInput` (`GameplayStatics.GetPlayerController` 0))
    (`self.Toggle_Pause_Game`)
    (else
      (set `self.Tutorial_Active?` false)
      (if (`self.Power_Drain_To_Resume?`)
        (set `self.Power_Drain_Active?` true)
        (set `self.Power_Drain_To_Resume?` false)))))

(event `Key|E` :paused true
  (params (Key :type "Key Structure"))
  (:`Released`
    (bind _foundwidgets (`WidgetBlueprintLibrary.GetAllWidgetsWithInterface` "/Game/Interface/Tooltips/Int_Tutorial_Interface.Int_Tutorial_Interface_C"))
    (for _array_element _foundwidgets
      (`Widget.RemoveFromParent` _array_element))
    (`self.DisableInput` (`GameplayStatics.GetPlayerController` 0))
    (`self.Toggle_Pause_Game`)))

(fn `PopUp_DisplayPoints_PowerDrain`
  (bind _returnvalue (`|CreateWidget` "/Game/Interface/Tooltips/Wid_Time_Display_Points.Wid_Time_Display_Points_C" (`self.Player_Ref`)))
  (`UserWidget.AddToViewport` _returnvalue 0)
  (`self.Toggle_Tutorial` true))

(fn `PopUp_DoubleJump_Slide`
  (bind _returnvalue (`|CreateWidget` "/Game/Interface/Tooltips/Wid_Double_Jump_Slide.Wid_Double_Jump_Slide_C" (`self.Player_Ref`)))
  (`UserWidget.AddToViewport` _returnvalue 0)
  (`self.Toggle_Tutorial` true))

(fn `PopUp_WallRun_Ghostflicker`
  (bind _returnvalue (`|CreateWidget` "/Game/Interface/Tooltips/Wid_Double_Jump_Slide.Wid_Double_Jump_Slide_C" (`self.Player_Ref`)))
  (`UserWidget.AddToViewport` _returnvalue 0)
  (`self.Toggle_Tutorial` true))

(fn `Toggle_Pause_Game`
  (if (`self.Paused?`)
    (set `self.Paused?` false)
    (`GameplayStatics.SetGamePaused` false)
    (else
      (set `self.Paused?` true)
      (`GameplayStatics.SetGamePaused` true))))

(fn `UserConstructionScript`)