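; BP_Display_Points is a level actor that acts as a healing point for the player.
; When a Player-tagged actor overlaps its Box, it casts the first player pawn to BP_Player_Character and restores 70% of missing health, truncated to an integer.
; It then deactivates the PKyMagicCircle1 effect, but the trigger stays enabled, so later overlaps heal again.
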(event `self.Box.OnComponentBeginOverlap`
  (params (OverlappedComponent :type "PrimitiveComponent Object Reference") (OtherActor :type "Actor Object Reference") (OtherComp :type "PrimitiveComponent Object Reference") (OtherBodyIndex :type Integer) (bFromSweep :type Boolean) (SweepResult :type "HitResult Structure (by ref)"))
  (if (`self.ActorHasTag` OtherActor "Player")
    (bind _asbp_player_character (cast `/Game/Player_Character/Blueprints/BP_Player_Character` (`GameplayStatics.GetPlayerPawn` 0)))
    (set `/Game/Player_Character/Blueprints/BP_Player_Character.Current_Health` (+ (`/Game/Player_Character/Blueprints/BP_Player_Character.Current_Health` _asbp_player_character) (`KismetMathLibrary.FTrunc` (* (- (`/Game/Player_Character/Blueprints/BP_Player_Character.Max_Health` _asbp_player_character) (`/Game/Player_Character/Blueprints/BP_Player_Character.Current_Health` _asbp_player_character)) 0.7))) _asbp_player_character)
    (`ActorComponent.Deactivate` (`self.P_ky_magicCircle1`))))

(fn `UserConstructionScript`)