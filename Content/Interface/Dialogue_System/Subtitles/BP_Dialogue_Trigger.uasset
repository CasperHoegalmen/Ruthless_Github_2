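; BP_Dialogue_Trigger is a volume actor that shows a subtitle dialogue widget while the player is inside its box.
; Begin and end overlaps from components tagged Player_Collider both call TriggerDialogue, which works as a toggle.
; It removes and clears an existing widget, or creates a Widget_Dialogue for player 0, adds it to the viewport and sets its DialogueText from SubtitleText.
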(event `self.Trigger Dialogue`
  (`/Engine/EditorBlueprintResources/StandardMacros.IsValid` (`self.Dialogue_Widget`)
    (:`Is Valid`
      (`Widget.RemoveFromParent` (`self.Dialogue_Widget`))
      (set `self.Dialogue_Widget` null))
    (:`Is Not Valid`
      (bind _returnvalue (`|CreateWidget` "/Game/Interface/Dialogue_System/Subtitles/Widget_Dialogue.Widget_Dialogue_C" (`GameplayStatics.GetPlayerController` 0)))
      (bind _output_get (set `self.Dialogue_Widget` _returnvalue))
      (`UserWidget.AddToViewport` _output_get 0)
      (set `/Game/Interface/Dialogue_System/Subtitles/Widget_Dialogue.Dialogue_Text` (`self.Subtitle_Text`) (`self.Dialogue_Widget`)))))

(event `self.Box.OnComponentBeginOverlap`
  (params (OverlappedComponent :type "PrimitiveComponent Object Reference") (OtherActor :type "Actor Object Reference") (OtherComp :type "PrimitiveComponent Object Reference") (OtherBodyIndex :type Integer) (bFromSweep :type Boolean) (SweepResult :type "HitResult Structure (by ref)"))
  (if (`ActorComponent.ComponentHasTag` OtherComp "Player_Collider")
    (`self.Trigger Dialogue`)))

(event `self.Box.OnComponentEndOverlap`
  (params (OverlappedComponent :type "PrimitiveComponent Object Reference") (OtherActor :type "Actor Object Reference") (OtherComp :type "PrimitiveComponent Object Reference") (OtherBodyIndex :type Integer))
  (if (`ActorComponent.ComponentHasTag` OtherComp "Player_Collider")
    (`self.Trigger Dialogue`)))

(fn `UserConstructionScript`)