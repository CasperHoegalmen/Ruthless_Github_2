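; Encounter zone actor that puts its BP_Unity_Rebel enemies into combat when the player enters it.
; An overlap of the EncounterVolume by a Player-tagged actor calls Call_Out_Target with the player pawn's current location.
; That event loops over all rebels, and for those overlapping this actor sets InCombat and writes the combat flag and target location to their AI blackboards.
; The location is a one-time snapshot per overlap, not continuously tracked.
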(event `Call_Out_Target`
  (params (Target_Location :type "Vector Structure"))
  (set `self.Target_Location` Target_Location)
  (bind _outactors (`GameplayStatics.GetAllActorsOfClass` "/Game/Enemies/Unity_Rebel/BP_Unity_Rebel.BP_Unity_Rebel_C"))
  (for _array_element _outactors
    (if (`self.IsOverlappingActor` _array_element)
      (bind _output_get (set `/Game/Enemies/Unity_Rebel/BP_Unity_Rebel.In_Combat?` true _array_element))
      (bind _returnvalue (`AIBlueprintHelperLibrary.GetBlackboard` _array_element))
      (`BlackboardComponent.SetValueAsBool` _returnvalue "In_Combat?" _output_get)
      (`BlackboardComponent.SetValueAsVector` _returnvalue "Target_Location" (`self.Target_Location`)))))

(event `self.EncounterVolume.OnComponentBeginOverlap`
  (params (OverlappedComponent :type "PrimitiveComponent Object Reference") (OtherActor :type "Actor Object Reference") (OtherComp :type "PrimitiveComponent Object Reference") (OtherBodyIndex :type Integer) (bFromSweep :type Boolean) (SweepResult :type "HitResult Structure (by ref)"))
  (if (`self.ActorHasTag` OtherActor "Player")
    (`self.Call_Out_Target` (`self.K2_GetActorLocation` (`GameplayStatics.GetPlayerPawn` 0)))))

(fn `UserConstructionScript`)