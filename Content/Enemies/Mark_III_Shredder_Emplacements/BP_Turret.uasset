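; BP_Turret is an enemy turret that turns to face the first-person player and shoots at them.
; PawnSensing's See Pawn event drives it, snapping the actor's rotation toward any sighted FirstPersonCharacter.
; It then spawns a FirstPersonProjectile at ProjectileSpawnLocation and launches it along the Cube's forward vector with a velocity-change impulse.
; A boolean gate reset after a short Delay limits the fire rate.
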(event `self.PawnSensing.OnSeePawn`
  (params (Pawn :type "Pawn Object Reference"))
  (bind _asfirst_person_character (cast `/Game/Player_Character/Blueprints/FirstPersonCharacter` Pawn))
  (`|ExecutionSequence`
    (:`then_0`
      (`self.K2_SetActorRotation` (`KismetMathLibrary.FindLookAtRotation` (`self.K2_GetActorLocation`) (`self.K2_GetActorLocation` _asfirst_person_character))))
    (:`then_1`
      (if (`self.Can_Spawn_Projectile?`)
        (bind _returnvalue (`|SpawnActorFromClass` "/Game/Player_Character/Blueprints/FirstPersonProjectile.FirstPersonProjectile_C" (`SceneComponent.K2_GetComponentToWorld` (`self.Projectile_Spawn_Location`)) "Undefined" "OverrideRootScale" null null))
        (`PrimitiveComponent.AddImpulse` (`/Game/Player_Character/Blueprints/FirstPersonProjectile.Sphere` _returnvalue) (* (`SceneComponent.GetForwardVector` (`self.Cube`)) (`self.Projectile_Velocity`)) "None" true)
        (set `self.Can_Spawn_Projectile?` false)
        (`KismetSystemLibrary.Delay` 0.8)
        (set `self.Can_Spawn_Projectile?` true)))))

(fn `UserConstructionScript`)